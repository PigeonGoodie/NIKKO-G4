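; BP_PedestrianPath is a spline path actor that lays out NPC_Point actors for pedestrians at runtime.
; On BeginPlay, PlaceNPCPoints spawns points every 400 units along the Path spline in world space and stores them in NpcPoint.
; Before spawning, it calls SetLifeSpan(0) on stored points, which does not destroy them, then clears the array.
; The construction script is empty, with an unconnected PlaceNPCPoints call left in it.
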(event `self.ReceiveBeginPlay`
  (`self.Place NPC Points`))

(event `Place NPC Points`
  (set `self.Distance` 0.0)
  (for _array_element (`self.NpcPoint`)
    (`self.SetLifeSpan` _array_element 0.0))
  (`KismetArrayLibrary.Array_Clear` (`self.NpcPoint`))
  (bind _returnvalue (`|SpawnActorFromClass` "/Game/Gruppe3/Blueprints/PedestrianBP/NPC_Point.NPC_Point_C" (`KismetMathLibrary.MakeTransform` (`SplineComponent.GetLocationAtDistanceAlongSpline` (`self.Path`) (`self.Distance`) "World")) "Undefined" "OverrideRootScale" null null :!label _label))
  (`KismetArrayLibrary.Array_Add` (`self.NpcPoint`) _returnvalue)
  (bind _output_get (set `self.Distance` (+ (`self.Distance`) 400.0)))
  (if (< _output_get (`SplineComponent.GetSplineLength` (`self.Path`)))
    (goto _label)))

(fn `UserConstructionScript`)