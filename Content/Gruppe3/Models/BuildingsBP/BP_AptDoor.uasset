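; BP_AptDoor is an automatic double sliding apartment door that opens when something overlaps its trigger box.
; On overlap it plays the door sound and runs two timelines that set the relative locations of the left and right door panels.
; When the overlap ends, it waits half a second, plays the sound more quietly and reverses both timelines to close the door.
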(event `self.Box.OnComponentBeginOverlap`
  (params (OverlappedComponent :type "PrimitiveComponent Object Reference") (OtherActor :type "Actor Object Reference") (OtherComp :type "PrimitiveComponent Object Reference") (OtherBodyIndex :type Integer) (bFromSweep :type Boolean) (SweepResult :type "HitResult Structure (by ref)"))
  (`GameplayStatics.PlaySound2D` "/Game/Gruppe3/Audio/Ambiance/SFX/Doors/ApartmentDoor.ApartmentDoor" 2.0 1.0 0.0 null null)
  (`|ExecutionSequence`
    (:`then_0`
      (bind (_direction _doorslidel) (`Timeline|DoorSlideR` :!label _label)
        (:`Update`
          (`SceneComponent.K2_SetRelativeLocation` (`self.DoorR`) _doorslidel false false))))
    (:`then_1`
      (bind (_direction_2 _doorslidel_2) (`Timeline|DoorslideL` :!label _label_2)
        (:`Update`
          (`SceneComponent.K2_SetRelativeLocation` (`self.DoorL`) _doorslidel_2 false false))))))

(event `self.Box.OnComponentEndOverlap`
  (params (OverlappedComponent :type "PrimitiveComponent Object Reference") (OtherActor :type "Actor Object Reference") (OtherComp :type "PrimitiveComponent Object Reference") (OtherBodyIndex :type Integer))
  (`KismetSystemLibrary.Delay` 0.5)
  (`GameplayStatics.PlaySound2D` "/Game/Gruppe3/Audio/Ambiance/SFX/Doors/ApartmentDoor.ApartmentDoor" 0.7 1.0 0.0 null null)
  (`|ExecutionSequence`
    (:`then_0`
      (goto _label :!via `Reverse`))
    (:`then_1`
      (goto _label_2 :!via `Reverse`))))

(fn `UserConstructionScript`)