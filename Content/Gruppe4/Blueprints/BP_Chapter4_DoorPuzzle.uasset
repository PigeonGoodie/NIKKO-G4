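; Key-and-door puzzle actor for Chapter 4 that holds both a collectible key and a locked sewer door.
; Overlapping the sphere grants the key, destroys its mesh and briefly shows a found-key widget.
; The box trigger shows an unlock or locked prompt depending on key possession.
; Interact, on press or release, only opens the door while the unlock prompt is visible, sliding it to a second door component's relative transform.
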(event `InputAction|Interact`
  (params (Key :type "Key Structure"))
  (bind _as_widget_bp_unlock_door (`self.As Widget BP Unlock Door`))
  (bind _sm_sewer_door1 (`self.SM_Sewer_Door1`))
  (:`Pressed`
    (`KismetSystemLibrary.PrintString` "Interaction Pressed" :!label _label)
    (`/Engine/EditorBlueprintResources/StandardMacros.IsValid` _as_widget_bp_unlock_door
      (:`Is Valid`
        (if (`self.Door Is Open`)
          _
          (elif (`Widget.IsInViewport` _as_widget_bp_unlock_door)
            (`Widget.RemoveFromParent` _as_widget_bp_unlock_door)
            (set `self.Door Is Open` true)
            (`KismetSystemLibrary.MoveComponentTo` (`self.SM_Sewer_Door`) (`SceneComponent.RelativeLocation` _sm_sewer_door1) (`SceneComponent.RelativeRotation` _sm_sewer_door1) false false 5.0))))
      (:`Is Not Valid`
        (`KismetSystemLibrary.PrintString` "Button Prompt Is Not Active"))))
  (:`Released`
    (goto _label)))

(event `self.ReceiveBeginPlay`
  (`self.EnableInput` (`GameplayStatics.GetPlayerController` 0)))

(event `self.Box.OnComponentBeginOverlap`
  (params (OverlappedComponent :type "PrimitiveComponent Object Reference") (OtherActor :type "Actor Object Reference") (OtherComp :type "PrimitiveComponent Object Reference") (OtherBodyIndex :type Integer) (bFromSweep :type Boolean) (SweepResult :type "HitResult Structure (by ref)"))
  (if (`self.Door Is Open`)
    _
    (elif (`self.Has Key`)
      (bind _returnvalue (`|CreateWidget` "/Game/Gruppe4/Blueprints/Widget_BP_unlockDoor.Widget_BP_unlockDoor_C"))
      (bind _output_get (set `self.As Widget BP Unlock Door` _returnvalue))
      (`UserWidget.AddToViewport` _output_get 0)
      (else
        (bind _returnvalue_2 (`|CreateWidget` "/Game/Gruppe4/Blueprints/Widget_BP_doorIsLocked.Widget_BP_doorIsLocked_C"))
        (bind _output_get_2 (set `self.As Widget BP Door Is Locked` _returnvalue_2))
        (`UserWidget.AddToViewport` _output_get_2 0)))))

(event `self.Box.OnComponentEndOverlap`
  (params (OverlappedComponent :type "PrimitiveComponent Object Reference") (OtherActor :type "Actor Object Reference") (OtherComp :type "PrimitiveComponent Object Reference") (OtherBodyIndex :type Integer))
  (bind _as_widget_bp_door_is_locked (`self.As Widget BP Door Is Locked`))
  (bind _as_widget_bp_unlock_door (`self.As Widget BP Unlock Door`))
  (if (`Widget.IsInViewport` _as_widget_bp_unlock_door)
    (`Widget.RemoveFromParent` _as_widget_bp_unlock_door)
    (elif (`KismetSystemLibrary.IsValid` _as_widget_bp_door_is_locked)
      (if (`Widget.IsInViewport` _as_widget_bp_door_is_locked)
        (`Widget.RemoveFromParent` _as_widget_bp_door_is_locked)))))

(event `self.Sphere.OnComponentBeginOverlap`
  (params (OverlappedComponent :type "PrimitiveComponent Object Reference") (OtherActor :type "Actor Object Reference") (OtherComp :type "PrimitiveComponent Object Reference") (OtherBodyIndex :type Integer) (bFromSweep :type Boolean) (SweepResult :type "HitResult Structure (by ref)"))
  (if (not (stale _output_get_2))
    (bind _returnvalue (`|CreateWidget` "/Game/Gruppe4/Blueprints/Widget_BP_foundKey.Widget_BP_foundKey_C"))
    (bind _output_get (set `self.As Widget BP Found Key` _returnvalue))
    (`UserWidget.AddToViewport` _output_get 0)
    (bind _output_get_2 (set `self.Has Key` true))
    (`ActorComponent.K2_DestroyComponent` (`self.SM_Key`))
    (`KismetSystemLibrary.PrintString` "Key found and destroyed")
    (`KismetSystemLibrary.Delay` 2.0)
    (if (`Widget.IsInViewport` _output_get)
      (`Widget.RemoveFromParent` _output_get))))

(fn `UserConstructionScript`)