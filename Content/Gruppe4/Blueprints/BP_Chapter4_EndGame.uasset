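; Chapter 4 end-game trigger actor that lets the player start the end credits from an interaction prompt.
; Overlapping its collision component shows a button prompt widget, and leaving removes it.
; Interact or E, on both press and release, runs one shared path that, while the prompt is in the viewport, disables player movement and plays the credit roll widget.
; A level sequence playback step before the credits is switched off by a constant false branch.
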(event `self.CollisionComponent.OnComponentBeginOverlap`
  (params (OverlappedComponent :type "PrimitiveComponent Object Reference") (OtherActor :type "Actor Object Reference") (OtherComp :type "PrimitiveComponent Object Reference") (OtherBodyIndex :type Integer) (bFromSweep :type Boolean) (SweepResult :type "HitResult Structure (by ref)"))
  (`self.EnableInput` null)
  (bind _returnvalue (`|CreateWidget` "/Game/Gruppe4/Blueprints/Widget_BP_buttonPromptEndCredits.Widget_BP_buttonPromptEndCredits_C"))
  (bind _output_get (set `self.NewVar_0` _returnvalue))
  (`UserWidget.AddToViewport` _output_get 0))

(event `self.CollisionComponent.OnComponentEndOverlap`
  (params (OverlappedComponent :type "PrimitiveComponent Object Reference") (OtherActor :type "Actor Object Reference") (OtherComp :type "PrimitiveComponent Object Reference") (OtherBodyIndex :type Integer))
  (`Widget.RemoveFromParent` (stale `self.CollisionComponent.OnComponentBeginOverlap` _output_get)))

(event `InputAction|Interact`
  (params (Key :type "Key Structure"))
  (:`Pressed`
    (`KismetSystemLibrary.PrintString` "Interaction Pressed" :!label _label)
    (`/Engine/EditorBlueprintResources/StandardMacros.IsValid` (stale `self.CollisionComponent.OnComponentBeginOverlap` _output_get)
      (:`Is Valid`
        (if (`Widget.IsInViewport` (stale `self.CollisionComponent.OnComponentBeginOverlap` _output_get))
          (`/Game/StoryAdvTemplate/Blueprints/Core/BP_StoryAdv_FunctionLibrary.DisablePlayerMovement`)
          (`Widget.RemoveFromParent` (stale `self.CollisionComponent.OnComponentBeginOverlap` _output_get))
          (if false
            (bind _outactor (`LevelSequencePlayer.CreateLevelSequencePlayer` "/Game/Gruppe4/LevelSequences/Greybox1_TestSequence.Greybox1_TestSequence"))
            (bind _sequenceplayer (`LevelSequenceActor.SequencePlayer` _outactor))
            (`MovieSceneSequencePlayer.SetPlaybackPosition` :`self` _sequenceplayer)
            (`MovieSceneSequencePlayer.Play` _sequenceplayer)
            (`KismetSystemLibrary.Delay` (`TimeManagementBlueprintLibrary.Conv_QualifiedFrameTimeToSeconds` (`MovieSceneSequencePlayer.GetDuration` _sequenceplayer))))
          (bind _returnvalue (`|CreateWidget` "/Game/Gruppe4/Blueprints/Widget_BP_endCredits.Widget_BP_endCredits_C"))
          (bind _output_get (set `self.NewVar_1` _returnvalue))
          (`UserWidget.AddToViewport` _output_get 0)
          (`UserWidget.PlayAnimation` _output_get (`/Game/Gruppe4/Blueprints/Widget_BP_endCredits.credit_roll` _output_get) 1.0 1 "Forward" 1.0 false)))
      (:`Is Not Valid`
        (`KismetSystemLibrary.PrintString` "Button Prompt Is Not Active"))))
  (:`Released`
    (goto _label)))

(event `Key|E`
  (params (Key :type "Key Structure"))
  (:`Pressed`
    (goto _label))
  (:`Released`
    (goto _label)))

(event `self.ReceiveBeginPlay`
  (`self.EnableInput` (`GameplayStatics.GetPlayerController` 0)))

(fn `UserConstructionScript`)