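; Configurable window blinds prop, built procedurally in the construction script from width, drop, slat width and open/close percentage.
; The frame stretches to the width, and the slat count follows from drop and slat width.
; Each spawned slat is scaled, rotated and either spaced or stacked at folding thickness, with two ropes scaled to the last slat.
; Dynamic material instances expose colour and surface settings, plus texture for slats.
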(fn `Metallic Setup`
  (params (IsMetallic :type Boolean) (Material :type "MaterialInstanceDynamic Object Reference"))
  (if IsMetallic
    (`MaterialInstanceDynamic.SetScalarParameterValue` Material "Metallic" 1.0)
    (else
      (`MaterialInstanceDynamic.SetScalarParameterValue` Material "Metallic" 0.0))))

(fn `UserConstructionScript`
  (bind _rope_shift (`self.rope Shift`))
  (bind _returnvalue (- (- (- (+ (+ (`self.location`) (`self.slat_width_var`)) (`self.Shift Vertical`)) (`self.shift`)) 4.0) (`self.Slat Width`)))
  (set `self.slat_width_var` (* (`self.Slat Width`) 0.8))
  (set `self.number of pieces` (`KismetMathLibrary.FFloor` (/ (`KismetMathLibrary.Conv_IntToDouble` (`self.Drop`)) (`self.slat_width_var`))))
  (set `self.fully folded size` (* (`self.number of pieces`) (`self.folding_dimension`)))
  (set `self.opening_var` (* (/ (`self.Open-Close`) 100.0) (`KismetMathLibrary.Conv_IntToDouble` (`self.Drop`))))
  (if (> (`self.opening_var`) (`self.fully folded size`))
    (set `self.shift` (`self.opening_var`))
    (else
      (set `self.shift` (`self.fully folded size`))))
  (`SceneComponent.SetRelativeScale3D` (`self.middle`) (`KismetMathLibrary.MakeVector` (/ (`KismetMathLibrary.Conv_IntToDouble` (`self.Width`)) 96.0) 1.0 1.0))
  (`SceneComponent.K2_SetRelativeLocation` (`self.end`) (`KismetMathLibrary.MakeVector` (- (`KismetMathLibrary.Conv_IntToDouble` (`self.Width`)) 96.0)) false false)
  (bind _returnvalue_2 (`AddComponent|NODE_AddStaticMeshComponent-0`))
  (set `self.rope left` _returnvalue_2)
  (bind _returnvalue_3 (`AddComponent|NODE_AddStaticMeshComponent-1`))
  (set `self.rope right` _returnvalue_3)
  (bind _returnvalue_4 (`KismetMaterialLibrary.CreateDynamicMaterialInstance` null))
  (set `self.Frame Material` _returnvalue_4)
  (`PrimitiveComponent.SetMaterial` (`self.middle`) 0 (`self.Frame Material`))
  (`PrimitiveComponent.SetMaterial` (`self.end`) 0 (`self.Frame Material`))
  (`PrimitiveComponent.SetMaterial` (`self.start`) 0 (`self.Frame Material`))
  (bind _returnvalue_5 (`KismetMaterialLibrary.CreateDynamicMaterialInstance` null))
  (set `self.Rope Material` _returnvalue_5)
  (`PrimitiveComponent.SetMaterial` (`self.rope left`) 0 (`self.Rope Material`))
  (`PrimitiveComponent.SetMaterial` (`self.rope right`) 0 (`self.Rope Material`))
  (`MaterialInstanceDynamic.SetVectorParameterValue` (`self.Frame Material`) "Base Colour" (`self.Frame Colour`))
  (`self.Metallic Setup` (`self.Frame Metallic`) (`self.Frame Material`))
  (`MaterialInstanceDynamic.SetScalarParameterValue` (`self.Frame Material`) "Roughness" (`self.Frame Roughness`))
  (`MaterialInstanceDynamic.SetScalarParameterValue` (`self.Frame Material`) "Specular" (`self.Frame Specular`))
  (`MaterialInstanceDynamic.SetVectorParameterValue` (`self.Rope Material`) "Base Colour" (`self.Rope Colour`))
  (for _index (range (+ (`self.number of pieces`) 1))
    (set `self.slat index` (- (`self.number of pieces`) _index))
    (if (< (`self.opening_var`) (`self.fully folded size`))
      (set `self.location` (* (`self.slat index`) (`self.folding_dimension`)))
      (else
        (set `self.location` (`self.opening_var`))
        (set `self.fully folded size` (- (`self.fully folded size`) (`self.folding_dimension`)))
        (set `self.opening_var` (- (`self.location`) (`self.slat_width_var`)))))
    (bind _returnvalue_6 (`AddComponent|NODE_AddStaticMeshComponent-2`))
    (set `self.Slat` _returnvalue_6)
    (bind _returnvalue_7 (`PrimitiveComponent.CreateDynamicMaterialInstance` (`self.Slat`) 0 null "None"))
    (set `self.Slat Material` _returnvalue_7)
    (`MaterialInstanceDynamic.SetTextureParameterValue` (`self.Slat Material`) "Base Colour" (`self.Slat Texture`))
    (`MaterialInstanceDynamic.SetVectorParameterValue` (`self.Slat Material`) "Tint" (`self.Slat Colour`))
    (`MaterialInstanceDynamic.SetScalarParameterValue` (`self.Slat Material`) "Brightness" (`self.Slat Brightness`))
    (`MaterialInstanceDynamic.SetScalarParameterValue` (`self.Slat Material`) "Contrast" (`self.Slat Contrast`))
    (`self.Metallic Setup` (`self.Slat Metallic`) (`self.Slat Material`))
    (`MaterialInstanceDynamic.SetScalarParameterValue` (`self.Slat Material`) "Specular" (`self.Slat Specular`))
    (`MaterialInstanceDynamic.SetScalarParameterValue` (`self.Slat Material`) "Roughness" (`self.Slat Roughness`))
    (set `self.rope Shift` _returnvalue)
    (`SceneComponent.K2_SetRelativeLocation` (`self.Slat`) (`KismetMathLibrary.MakeVector` 0.0 0.0 _returnvalue) false false)
    (`SceneComponent.SetRelativeScale3D` (`self.Slat`) (`KismetMathLibrary.MakeVector` (/ (`KismetMathLibrary.Conv_IntToDouble` (`self.Width`)) 96.0) (/ (`self.Slat Width`) 5.0) 1.0))
    (`SceneComponent.K2_SetRelativeRotation` (`self.Slat`) (`KismetMathLibrary.MakeRotator` (`KismetMathLibrary.Conv_IntToDouble` (+ (`self.Slat Rotation`) -90))) false false)
    (if (== (`self.slat index`) 0)
      (`SceneComponent.K2_SetRelativeLocation` (`self.rope left`) (`KismetMathLibrary.MakeVector` 10.0 0.0 _rope_shift) false false)
      (`SceneComponent.K2_SetRelativeLocation` (`self.rope right`) (`KismetMathLibrary.MakeVector` (`KismetMathLibrary.Conv_IntToDouble` (- (`self.Width`) 10)) 0.0 _rope_shift) false false)
      (`SceneComponent.SetRelativeScale3D` (`self.rope left`) (`KismetMathLibrary.MakeVector` 1.0 1.0 (/ (* (- _rope_shift -1.0) -1.0) 99.0)))
      (`SceneComponent.SetRelativeScale3D` (`self.rope right`) (`KismetMathLibrary.MakeVector` 1.0 1.0 (/ (* (- _rope_shift -1.0) -1.0) 99.0))))))